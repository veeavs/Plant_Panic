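; BP_Plant is a potted plant actor with health, a random plant mesh picked at BeginPlay, and a WaterLevel health bar that turns toward the player each tick.
; Damage lowers health, and StartDOT and EndDOT control a one-second looping timer that reapplies the last damage received.
; At zero health it destroys itself, plays a sound and damages the player character to feed the panic meter.
; Outline and random-pot logic are unconnected.
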(event OnBeginCursorOver(PlantCube)
  (params (TouchedComponent :type Primitive%20Component%20Object%20Reference)))

(event Custom|StartDOT
  ;[1 0.1094 0.1094] Damage to plants
  (bind _returnvalue (Utilities|Time|SetTimerbyEvent (delegate Custom|DOT) 1.0 true))
  (Variables|Default|SetDOT_timer _returnvalue))

(event Custom|DOT
  ;[1 0.1094 0.1094] Damage to plants
  (Game|Damage|ApplyDamage self (Variables|Default|GetDamagedReceived) 0 0))

(event Custom|EndDOT
  ;[1 0.1094 0.1094] Damage to plants
  ;;[1 1 1] stops timer from running
  (Utilities|Time|ClearandInvalidateTimerbyHandle (Variables|Default|GetDOT_timer)))

(event EventBeginPlay
  ;[0.4327 0.3558 1] Randomize Plant Mesh
  (Components|StaticMesh|SetStaticMesh (Variables|Default|Getbotanical) (.OutItem (Utilities|Array|Random (Utilities|Array|MakeArray "/Game/Plants/MBJ_PlantPack01_Plant04v001.MBJ_PlantPack01_Plant04v001" "/Game/Plants/MBJ_PlantPack01_Plant05v001.MBJ_PlantPack01_Plant05v001" "/Game/Plants/MBJ_PlantPack01_Plant01v001.MBJ_PlantPack01_Plant01v001" "/Game/Plants/MBJ_PlantPack01_Plant02v001.MBJ_PlantPack01_Plant02v001" "/Game/Plants/MBJ_PlantPack01_Plant03v001.MBJ_PlantPack01_Plant03v001")))))

(event EventTick
  (params (DeltaSeconds :type Float%20%28single-precision%29))
  ;[1 1 1] Rotate health bar to always face player
  (Transformation|SetWorldRotation (Variables|Default|GetWater%20Level) (Math|Rotator|FindLookatRotation (Transformation|GetWorldLocation (Variables|Default|GetWater%20Level)) (Transformation|GetActorLocation (Game|GetPlayerCharacter 0))) false false))

(event Game|Damage|EventAnyDamage
  (params (Damage :type Float%20%28single-precision%29) (DamageType :type Damage%20Type%20Object%20Reference) (InstigatedBy :type Controller%20Object%20Reference) (DamageCauser :type Actor%20Object%20Reference))
  ;[1 0.1094 0.1094] Damage to plants
  (bind _output_get (Variables|Default|SetDamagedReceived Damage))
  (bind _output_get_2 (Variables|Default|SetHealthPlant (- (Variables|Default|GetHealthPlant) _output_get)))
  (if (<= _output_get_2 0.0)
    (Actor|DestroyActor)
    (Audio|PlaySound2D "/Game/Sounds/703249__xkeril__magic-attack-small.703249__xkeril__magic-attack-small" 1.0 1.0 0.0 0 0)
    ;;[0.9184 0.1189 1] Damage Player (Panic Meter)
    (bind _returnvalue (Actor|GetActorOfClass "/Game/ThirdPerson/Blueprints/BP_ThirdPersonCharacter.BP_ThirdPersonCharacter_C"))
    (Game|Damage|ApplyDamage _returnvalue 1e+01 0 0)))

(fn ConstructionScript)

(fn PlantRef
  (return self))